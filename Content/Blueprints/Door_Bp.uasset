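; Door actor that the third-person character can open and close with the Interact input, provided it has a key.
; Overlapping the box shows an interact widget, enables input and opens a gate; leaving reverses all three.
; With the key, a FlipFlop alternately plays and reverses a timeline that lerps the mesh's yaw between closed and open angles.
; Without it, a locked-door sound plays.
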(event OnComponentBeginOverlap(Box)
  (params (OverlappedComponent :type Primitive%20Component%20Object%20Reference) (OtherActor :type Actor%20Object%20Reference) (OtherComp :type Primitive%20Component%20Object%20Reference) (OtherBodyIndex :type Integer) (bFromSweep :type Boolean) (SweepResult :type Hit%20Result%20Structure%20%28by%20ref%29))
  ;[1 1 1] Open/Close Door
  (bind _asbp_third_person_character (Utilities|Casting|CastToBP_ThirdPersonCharacter OtherActor))
  (bind _returnvalue (UserInterface|CreateWidget "/Game/Widgets/Interact_Wd1.Interact_Wd1_C"))
  (UserInterface|Viewport|AddtoViewport _returnvalue 0)
  (Input|EnableInput (Game|GetPlayerController 0))
  (Utilities|FlowControl|Gate true) ; enters at Open
)

(event OnComponentEndOverlap(Box)
  (params (OverlappedComponent :type Primitive%20Component%20Object%20Reference) (OtherActor :type Actor%20Object%20Reference) (OtherComp :type Primitive%20Component%20Object%20Reference) (OtherBodyIndex :type Integer))
  ;[1 1 1] Open/Close Door
  (Utilities|Casting|CastToBP_ThirdPersonCharacter OtherActor)
  (Widget|RemovefromParent (stale OnComponentBeginOverlap(Box) _returnvalue))
  (Input|DisableInput (Game|GetPlayerController 0))
  (Utilities|FlowControl|Gate true) ; enters at Close
)

(event Input|ActionEvents|InputActionInteract
  (params (Key :type Key%20Structure :default "None"))
  ;[1 1 1] Open/Close Door
  (:Pressed
    (if (Variables|/Game/ThirdPerson/Blueprints/BP_ThirdPersonCharacter.BP_ThirdPersonCharacter_C|GetHasKey (stale OnComponentBeginOverlap(Box) _asbp_third_person_character))
      (Utilities|FlowControl|Gate true
        (:Exit
          (Utilities|FlowControl|FlipFlop
            (:A
              (bind _door_track (Timeline|OpenDoor Play)
                (:Update
                  (Transformation|SetRelativeRotation (Variables|Default|GetStaticMesh) (Math|Rotator|MakeRotator 0.0 0.0 (Math|Float|Lerp (Variables|Default|GetClosedAngle) (Variables|Default|GetOpenAngle) _door_track)) false false))))
            (:B
              (Timeline|OpenDoor Reverse)))))
      (else
        (Audio|PlaySoundatLocation "/Game/Sound/door_locked.door_locked" (Transformation|GetActorLocation) "0, 0, 0" 1.0 1.0 0.0 0 0 0 0)))))

(fn ConstructionScript)